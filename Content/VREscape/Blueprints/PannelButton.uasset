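; PannelButton is an interactable panel button that signals connected door objects when pressed while powered.
; An overlap box enables player input while a BP_MotionController is inside and disables it on exit, using player controller 0 as a single-player placeholder.
; Both the FPSInteract action and the Interact event check IsPowered, then call CallEventsDoor, which passes ConnectedObjects to CommunicateOutputDoor.
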(event OnComponentBeginOverlap(Box)
  (params (OverlappedComponent :type Primitive%20Component%20Object%20Reference) (OtherActor :type Actor%20Object%20Reference) (OtherComp :type Primitive%20Component%20Object%20Reference) (OtherBodyIndex :type Integer) (bFromSweep :type Boolean) (SweepResult :type Hit%20Result%20Structure%20%28by%20ref%29))
  ;[1 1 1] Checks overlap for interact
  (Utilities|Casting|CastToBP_MotionController OtherActor)
  (Input|EnableInput (Game|GetPlayerController 0)))

(event OnComponentEndOverlap(Box)
  (params (OverlappedComponent :type Primitive%20Component%20Object%20Reference) (OtherActor :type Actor%20Object%20Reference) (OtherComp :type Primitive%20Component%20Object%20Reference) (OtherBodyIndex :type Integer))
  ;[1 1 1] Checks overlap for interact
  (Utilities|Casting|CastToBP_MotionController OtherActor)
  (Input|DisableInput (Game|GetPlayerController 0)))

(event Custom|CallEventsDoor
  ;[1 1 1] CallsDoorFunction
  (CallFunction|CommunicateOutputDoor (Variables|Default|GetConnectedObjects)))

(event Custom|Interact
  ;[1 1 1] Calls event if powered
  (if (Variables|Default|GetIsPowered?)
    (CallFunction|CallEventsDoor)))

(event Input|ActionEvents|InputActionFPSInteract
  (params (Key :type Key%20Structure))
  ;[1 1 1] Calls event if powered
  (:Pressed
    (if (Variables|Default|GetIsPowered?)
      (CallFunction|CallEventsDoor))))

(fn ConstructionScript)
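; Generator actor for a VR escape game that detects an electrified power cube and notifies its connected objects.
; A box overlap sets HasPowerCube when an InteractableObject with the electricity property enters, then fires GeneratorActivate.
; Any InteractableObject leaving the box clears the flag and fires the same event, regardless of its property.
; GeneratorActivate passes the ConnectedObjects and itself to CommunicateOutputGenerator.
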(event OnComponentBeginOverlap(Box)
  (params (OverlappedComponent :type Primitive%20Component%20Object%20Reference) (OtherActor :type Actor%20Object%20Reference) (OtherComp :type Primitive%20Component%20Object%20Reference) (OtherBodyIndex :type Integer) (bFromSweep :type Boolean) (SweepResult :type Hit%20Result%20Structure%20%28by%20ref%29))
  ;[1 1 1] Checks object has electricity
  (bind _asinteractable_object (Utilities|Casting|CastToInteractableObject OtherActor))
  (if (Utilities|Enum|Equal(Enum) (Variables|/Game/VREscape/Blueprints/InteractableObject.InteractableObject_C|GetProperty _asinteractable_object) "NewEnumerator4")
    ;[1 1 1] sets has power cube to true and triggers event
    (Variables|Default|SetHasPowerCube true)
    (CallFunction|GeneratorActivate)))

(event OnComponentEndOverlap(Box)
  (params (OverlappedComponent :type Primitive%20Component%20Object%20Reference) (OtherActor :type Actor%20Object%20Reference) (OtherComp :type Primitive%20Component%20Object%20Reference) (OtherBodyIndex :type Integer))
  ;[1 1 1] resets has power cube
  (Utilities|Casting|CastToInteractableObject OtherActor)
  (Variables|Default|SetHasPowerCube false)
  (CallFunction|GeneratorActivate))

(event Custom|GeneratorActivate
  ;[1 1 1] Communicates with function
  (CallFunction|CommunicateOutputGenerator (Variables|Default|GetConnectedObjects) self))

(fn ConstructionScript)
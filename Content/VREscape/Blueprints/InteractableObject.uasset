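; Interactable cube actor that reacts to being overlapped by a Projectile.
; Each projectile overlap flips between setting the Property enum to Null with the cube's material cleared, and assigning Property with CubeMaterial applied.
; BeginPlay switches on Property with no actions attached, and a lookup of the projectile's gun type is left unused.
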(event EventBeginPlay
  ;[1 1 1] Enum
  (switch Utilities|FlowControl|Switch|SwitchonWhichGun (Variables|Default|GetProperty)))

(event Collision|EventActorBeginOverlap
  (params (OtherActor :type Actor%20Object%20Reference))
  (bind _cube (Variables|Default|GetCube))
  (bind _asprojectile (Utilities|Casting|CastToProjectile OtherActor))
  (Utilities|FlowControl|FlipFlop
    (:A
      (Variables|Default|SetProperty "NewEnumerator0")
      (Rendering|Material|SetMaterial _cube 0 0))
    (:B
      (Variables|Default|SetProperty (Variables|Default|GetProperty))
      (Rendering|Material|SetMaterial _cube 0 "/Game/Geometry/Meshes/CubeMaterial.CubeMaterial"))))

(fn ConstructionScript)
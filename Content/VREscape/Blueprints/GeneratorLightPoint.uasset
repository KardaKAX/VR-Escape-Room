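; A generator-linked point light actor in a VR escape game that is lit only while powered.
; BeginPlay hides the PointLight, then Tick polls the IsPowered flag every frame.
; A DoOnce shows the light once on power-up; while unpowered, each tick hides it and resets the DoOnce.
; Nothing in this Blueprint sets IsPowered.
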(event EventBeginPlay
  ;[1 1 1] Sets light visbility
  (|CallParentFunction)
  (Rendering|SetVisibility (Variables|Default|GetPointLight) false false))

(event EventTick
  (params (DeltaSeconds :type Float%20%28single-precision%29))
  ;[1 1 1] Checks if power and sets visiblity
  (|CallParentFunction DeltaSeconds)
  (if (Variables|Default|GetIsPowered?)
    (Utilities|FlowControl|DoOnce false :!label _label
      (:Completed
        (Rendering|SetVisibility (Variables|Default|GetPointLight) true false)))
    (else
      (Utilities|FlowControl|Sequence
        (:then_0
          (Rendering|SetVisibility (Variables|Default|GetPointLight) false false))
        (:then_1
          (goto _label Reset))))))

(fn ConstructionScript
  (|CallParentFunction))
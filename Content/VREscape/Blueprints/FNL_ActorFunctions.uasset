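; Blueprint function library for the VR escape game that passes interactions on to connected actors.
; CommunicateOutputDoor casts each connected item to Door and toggles it open or closed based on its current state.
; CommunicateOutputGenerator casts each connected object to PannelButton and sets its powered state to match whether the generator holds a power cube.
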(fn CommunicateOutputDoor
  (params (ConnectedItems :type Array%20of%20Actor%20Object%20References))
  (for _array_element ConnectedItems
    (bind _asdoor (Utilities|Casting|CastToDoor _array_element))
    ;[1 1 1] checks if door is open, if true close, if false open
    (if (Variables|/Game/VREscape/Blueprints/Door.Door_C|GetOpen? _asdoor)
      (Default|DoorClose _asdoor)
      (else
        (Default|DoorOpen _asdoor)))))

(fn CommunicateOutputGenerator
  (params (ConnectedObjects :type Array%20of%20Actor%20Object%20References) (ActorSelf :type Generator%20Object%20Reference))
  (for _array_element ConnectedObjects
    ;[1 1 1] Set pannel to powered if generator has cube
    (bind _aspannel_button (Utilities|Casting|CastToPannelButton _array_element))
    (if (Variables|/Game/VREscape/Blueprints/Generator.Generator_C|GetHasPowerCube ActorSelf)
      (Variables|/Game/VREscape/Blueprints/PannelButton.PannelButton_C|SetIsPowered? _aspannel_button true)
      (else
        (Variables|/Game/VREscape/Blueprints/PannelButton.PannelButton_C|SetIsPowered? _aspannel_button false)))))
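; BP_Projectile is a VR escape game projectile that carries a property and takes on that property's material.
; On BeginPlay it updates its sphere's material from the instigating PlayerNoVR.
; A one-second delay then acts as a catchall for dodged shots: if it can target a player, it hands the current property to the targeted PlayerNoVR through PropertyReturned.
; The projectile destroys itself afterward, with no movement or hit logic in this graph.
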(event EventBeginPlay
  (Utilities|FlowControl|Sequence
    (:then_0
      ;[1 1 1] Give the projectile the material of the active property
      (bind _asplayer_no_vr (Utilities|Casting|CastToPlayerNoVR (Game|GetInstigator)))
      (CallFunction|UpdatePropertyMaterial _asplayer_no_vr (Variables|MyProjectile|GetSphere)))
    (:then_1
      ;[1 1 1] Catchall if the player dodges the projectile
      (Utilities|FlowControl|Delay 1.0)
      (if (Variables|Default|GetcanTargetPlayer)
        (bind _asplayer_no_vr_2 (Utilities|Casting|CastToPlayerNoVR (Variables|Default|GettargetedPlayer)))
        (Default|PropertyReturned _asplayer_no_vr_2 (Variables|Default|GetcurrentProperty))
        (Actor|DestroyActor)
        (else
          ;[1 1 1] Cleanup
          (Actor|DestroyActor))))))

(fn ConstructionScript)
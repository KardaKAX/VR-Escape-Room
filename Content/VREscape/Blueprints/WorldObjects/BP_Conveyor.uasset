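; Conveyor world object that procedurally builds a row of spline mesh segments, likely rollers, from editable count, spacing, length and size.
; The construction script adds segments spaced along local Y, and ConveyorSegmentSettings centres each one along X and scales its ends.
; A TL_ConveyorRotate timeline update would spin every stored segment through a full turn, but nothing in this graph starts it.
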(fn ConstructionScript
  (for _index (range 1 (Variables|Default|GetnumSegments))
    (bind _returnvalue (AddComponent|AddSplineMeshComponent false (Math|Transform|MakeTransform (Math|Vector|MakeVector 0.0 (* (- _index 1) (Variables|Default|GetconveyorSpacer)) 0.0) "0, 0, 0" "1,1,1")))
    (Utilities|Array|Add (Variables|Default|GetcreatedSplineMeshes) _returnvalue)
    (CallFunction|ConveyorSegmentSettings _returnvalue)))

(fn ConveyorSegmentSettings
  (params (splineMeshReference :type Spline%20Mesh%20Component%20Object%20Reference))
  (bind _conveyorlength (Variables|Default|GetconveyorLength))
  (bind _conveyorsize (Variables|Default|GetconveyorSize))
  (bind _returnvalue (/ _conveyorlength 2.0))
  (SplineMesh|SetStartPosition splineMeshReference (Math|Vector|MakeVector (* _returnvalue -1.0) 0.0 0.0) true)
  (SplineMesh|SetEndPosition splineMeshReference (Math|Vector|MakeVector _returnvalue 0.0 0.0) true)
  (SplineMesh|SetStartScale splineMeshReference (Math|Vector2D|MakeVector2D _conveyorsize _conveyorsize) true :!class /Script/Engine.SplineMeshComponent)
  (SplineMesh|SetEndScale splineMeshReference (Math|Vector2D|MakeVector2D _conveyorsize _conveyorsize) true :!class /Script/Engine.SplineMeshComponent))
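; BP_EffectCube is a physics puzzle cube that takes on a property from the first BP_Projectile that hits it.
; Properties lift it to a traced ceiling, split it into half-size copies, let pawns pass through, freeze it, enable input-driven resizing, or fire an Electrify dispatcher.
; WithdrawProperty reverts most effects, restores the stored material and spawns a return projectile targeting the originating player.
; A failed anti-gravity trace withdraws the property automatically.
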(event OnComponentHit(Cube)
  (params (HitComponent :type Primitive%20Component%20Object%20Reference) (OtherActor :type Actor%20Object%20Reference) (OtherComp :type Primitive%20Component%20Object%20Reference) (NormalImpulse :type Vector :default "0, 0, 0") (Hit :type Hit%20Result%20Structure%20%28by%20ref%29))
  ;[1 1 1] Check collisions and existing property
  (bind _asbp_projectile (Utilities|Casting|CastToBP_Projectile OtherActor))
  (if (Utilities|Enum|Equal(Enum) (Variables|Properties|GetpropertyCurrent) "NewEnumerator0")
    ;[1 1 1] Property application
    (Variables|Properties|SetpropertyCurrent (Variables|/Game/VREscape/Blueprints/BP_Projectile.BP_Projectile_C|GetcurrentProperty _asbp_projectile))
    (bind _output_get (Variables|Data|SetpropertyOriginActor (Variables|/Script/Engine.Actor|GetInstigator _asbp_projectile)))
    (Actor|DestroyActor _asbp_projectile)
    (bind _previousmaterial (CallFunction|UpdatePropertyMaterial _output_get (Variables|Default|GetCube)))
    (Variables|Data|SetstoredMaterial _previousmaterial)
    (bind _asplayer_no_vr (Utilities|Casting|CastToPlayerNoVR _output_get))
    (Default|PropertyFired _asplayer_no_vr)
    (switch Utilities|FlowControl|Switch|SwitchonEN_PropertyType (Variables|Properties|GetpropertyCurrent)
      (:NewEnumerator1
        (CallFunction|PropertyEventAntiGrav true))
      (:NewEnumerator2
        (CallFunction|PropertyEventDuplicate true))
      (:NewEnumerator3
        (Default|CallPropertyDispatcherElectrify))
      (:NewEnumerator6
        (CallFunction|PropertyEventPhase true))
      (:NewEnumerator7
        (CallFunction|PropertyEventScale true (Game|GetPlayerController 0)))
      (:NewEnumerator8
        (CallFunction|PropertyEventSuspend true)))))

(event Custom|Withdraw%20Property
  (params (callingActor :type Actor%20Object%20Reference))
  (bind _returnvalue (Transformation|GetActorLocation))
  (bind _propertycurrent (Variables|Properties|GetpropertyCurrent))
  ;[1 1 1] Property Withdrawl
  (bind _asplayer_no_vr (Utilities|Casting|CastToPlayerNoVR callingActor))
  (Variables|/Game/VREscape/Characters/PlayerNoVR.PlayerNoVR_C|SetisRetrievingShot _asplayer_no_vr true)
  (bind _returnvalue_2 (Game|SpawnActorfromClass "/Game/VREscape/Blueprints/BP_Projectile.BP_Projectile_C" (Math|Transform|MakeTransform _returnvalue (Math|Rotator|FindLookatRotation _returnvalue (Transformation|GetWorldLocation (select (Variables|/Game/VREscape/Characters/PlayerNoVR.PlayerNoVR_C|GetshotSecondary _asplayer_no_vr) (Variables|/Game/VREscape/Characters/PlayerNoVR.PlayerNoVR_C|GetGun_1P_R_ShotOrigin _asplayer_no_vr) (Variables|/Game/VREscape/Characters/PlayerNoVR.PlayerNoVR_C|GetGun_1P_L_ShotOrigin _asplayer_no_vr)))) "1,1,1") "AlwaysSpawn" 0 0))
  (bind _output_get (Variables|Data|SetreturnProjectile _returnvalue_2))
  (Variables|/Game/VREscape/Blueprints/BP_Projectile.BP_Projectile_C|SetcanTargetPlayer _output_get true)
  (Variables|/Game/VREscape/Blueprints/BP_Projectile.BP_Projectile_C|SettargetedPlayer _output_get (Variables|Data|GetpropertyOriginActor))
  (Collision|SetCollisionResponsetoAllChannels (Variables|/Game/VREscape/Blueprints/BP_Projectile.BP_Projectile_C|GetCollisionComponent _output_get) "ECR_Ignore")
  (Utilities|FlowControl|Sequence
    (:then_0
      (switch Utilities|FlowControl|Switch|SwitchonEN_PropertyType _propertycurrent
        (:NewEnumerator1
          (CallFunction|PropertyEventAntiGrav false))
        (:NewEnumerator2
          (CallFunction|PropertyEventDuplicate false))
        (:NewEnumerator6
          (CallFunction|PropertyEventPhase false))
        (:NewEnumerator7
          (CallFunction|PropertyEventScale false (Game|GetPlayerController 0)))
        (:NewEnumerator8
          (CallFunction|PropertyEventSuspend false))))
    (:then_1
      (Variables|/Game/VREscape/Blueprints/BP_Projectile.BP_Projectile_C|SetcurrentProperty (Variables|Data|GetreturnProjectile) _propertycurrent)
      (CallFunction|UpdatePropertyMaterial self (Variables|/Game/VREscape/Blueprints/BP_Projectile.BP_Projectile_C|GetSphere _output_get))
      (Rendering|Material|SetMaterial (Variables|Default|GetCube) 0 (Variables|Data|GetstoredMaterial))
      (Utilities|FlowControl|Delay 0.1)
      (Collision|SetCollisionResponsetoAllChannels (Variables|/Game/VREscape/Blueprints/BP_Projectile.BP_Projectile_C|GetCollisionComponent _output_get) "ECR_Block"))))

(event Custom|propertyEvent_Duplicate
  (params (isActive :type Boolean))
  (bind _self self)
  (bind _cube (Variables|Default|GetCube))
  ;[1 1 1] Duplicate
  (if isActive
    ;;[1 1 1] Effect Active
    (if (Utilities|Enum|NotEqual(Enum) (Variables|Properties|GetpropertyScale) "NewEnumerator0")
      (bind _returnvalue (Game|SpawnActorfromClass "BP_EffectCube_C" (Transformation|GetActorTransform) "AdjustIfPossibleButAlwaysSpawn" 0 0))
      (Variables|BP_EffectCube_C|SetpropertyCurrent _returnvalue "NewEnumerator2")
      (Variables|BP_EffectCube_C|SetpropertyScale _returnvalue (Utilities|Enum|ByteToEnumEN_PropertyScale (- (Variables|Properties|GetpropertyScale) 1)))
      (Variables|Properties|SetpropertyScale (Utilities|Enum|ByteToEnumEN_PropertyScale (- (Variables|Properties|GetpropertyScale) 1)))
      (Rendering|Material|SetMaterial (Variables|BP_EffectCube_C|GetCube _returnvalue) 0 "/Game/VREscape/Materials/Duplicate.Duplicate")
      (if (Utilities|Array|ContainsItem (Variables|Properties|Duplicate|Getduplicate_actorStorage) _self)
        _
        (else
          (Utilities|Array|Add (Variables|Properties|Duplicate|Getduplicate_actorStorage) _self)))
      (Utilities|Array|Add (Variables|Properties|Duplicate|Getduplicate_actorStorage) _returnvalue)
      (for _array_element (Variables|Properties|Duplicate|Getduplicate_actorStorage)
        (Variables|BP_EffectCube_C|Setduplicate_actorStorage _array_element (Variables|Properties|Duplicate|Getduplicate_actorStorage))
        (Variables|BP_EffectCube_C|SetstoredMaterial _array_element (Variables|Data|GetstoredMaterial))
        (Transformation|SetWorldScale3D (Variables|BP_EffectCube_C|GetCube _array_element) (* (Transformation|GetWorldScale (Variables|BP_EffectCube_C|GetCube _array_element)) 0.5))))
    (else
      ;;[1 1 1] Effect Inactive
      (Utilities|Array|RemoveItem (Variables|Properties|Duplicate|Getduplicate_actorStorage) self)
      (for _array_element_2 (Variables|Properties|Duplicate|Getduplicate_actorStorage)
        (Actor|DestroyActor _array_element_2))
      (Variables|Properties|SetpropertyScale (Utilities|Enum|ByteToEnumEN_PropertyScale (+ (Variables|Properties|GetpropertyScale) 1)))
      (Transformation|SetWorldScale3D _cube (* (Transformation|GetWorldScale _cube) 2.0))
      (Utilities|Array|Clear (Variables|Properties|Duplicate|Getduplicate_actorStorage)))))

(event Custom|propertyEvent_AntiGrav
  (params (isActive :type Boolean))
  (bind _returnvalue (Transformation|GetActorLocation))
  (bind _cube (Variables|Default|GetCube))
  (bind _boxextent (Collision|GetComponentBounds _cube))
  (bind _z (Math|Vector|BreakVector _boxextent))
  (bind _returnvalue_2 (/ _z 2.0))
  ;[1 1 1] Anti-Gravity
  (bind _enabled (CallFunction|IsDebug))
  (Physics|SetSimulatePhysics (Variables|Default|GetCube) (not isActive))
  (if isActive
    (Utilities|FlowControl|Sequence
      (:then_0
        (Utilities|FlowControl|DoOnce false
          (:Completed
            (Components|Timeline|SetPlayRate (Variables|Default|GetTL_Effect_AntiGrav_LiftAlpha) (/ 1.0 (Variables|Properties|AntiGravity|GetantiGrav_EffectTime))))))
      (:then_1
        (bind _outhit (Class|KismetSystemLibrary|BoxTraceSingleforObjects (+ _returnvalue (Math|Vector|MakeVector 0.0 0.0 _returnvalue_2)) (- (+ _returnvalue "0, 0,1000.000000") (Math|Vector|MakeVector 0.0 0.0 _returnvalue_2)) _boxextent (Math|Rotator|MakeRotator 0.0 0.0 (.yaw (Transformation|GetActorRotation))) (Utilities|Array|MakeArray "ObjectTypeQuery1") false 0 (select _enabled "Persistent" "None") true))
        (if (.bblockinghit _outhit)
          (bind _alpha (Timeline|TL_Effect_AntiGrav_LiftAlpha PlayFromStart)
            (:Update
              (Transformation|SetActorLocation (Math|Vector|Lerp(Vector) _returnvalue (.location _outhit) _alpha) false false)))
          (else
            (CallFunction|WithdrawProperty (Variables|Data|GetpropertyOriginActor))
            (|DebugGraph_TraceFailed _enabled)))))
    (else
      (Timeline|TL_Effect_AntiGrav_LiftAlpha Stop))))

(event Custom|propertyEvent_Suspend
  (params (isActive :type Boolean))
  ;[1 1 1] Suspend
  (Physics|SetSimulatePhysics (Variables|Default|GetCube) (not isActive)))

(event Custom|propertyEvent_Phase
  (params (isActive :type Boolean))
  ;[1 1 1] Phase
  (Collision|SetCollisionResponsetoChannel (Variables|Default|GetCube) "ECC_Pawn" (select isActive "ECR_Overlap" "ECR_Block")))

(event Custom|propertyEvent_Scale
  (params (isActive :type Boolean) (PlayerController :type Player%20Controller%20Object%20Reference))
  (bind _cube (Variables|Default|GetCube))
  ;[1 1 1] Phase
  (if isActive
    (Input|EnableInput PlayerController)
    (Utilities|FlowControl|Sequence
      (:then_0
        (Utilities|FlowControl|Gate true) ; enters at Open
      )
      (:then_1
        (Utilities|FlowControl|Gate true) ; enters at Open
      ))
    (else
      (Input|DisableInput PlayerController)
      (Utilities|FlowControl|Sequence
        (:then_0
          (Utilities|FlowControl|Gate true) ; enters at Close
        )
        (:then_1
          (Utilities|FlowControl|Gate true) ; enters at Close
        )))))

(event Input|ActionEvents|InputActionEffectIncrease
  (params (Key :type Key%20Structure))
  (bind _cube (Variables|Default|GetCube))
  ;[1 1 1] Phase
  (:Pressed
    (Utilities|FlowControl|Gate true
      (:Exit
        (bind _isa (Utilities|ExecutionCheck)
          (:Out%20A
            _)
          (:Out%20B
            _))
        (bind (_value _outofbounds_) (Utilities|CycleInteger -1 1 (select _isa 1 -1) false))
        (if (not _outofbounds_)
          (Variables|Properties|SetpropertyScale (Utilities|Enum|ByteToEnumEN_PropertyScale (Math|Conversions|ToByte(Integer) (+ _value 1))))
          (Transformation|SetWorldScale3D _cube (* (Transformation|GetWorldScale _cube) (select _isa 2.0 0.5)))
          (Transformation|AddActorWorldOffset (Math|Vector|MakeVector 0.0 0.0 (* (/ (.z (.BoxExtent (Collision|GetActorBounds false))) 2.0) (select _isa 1.0 -1.0)))))))))

(event Input|ActionEvents|InputActionEffectDecrease
  (params (Key :type Key%20Structure))
  (bind _cube (Variables|Default|GetCube))
  ;[1 1 1] Phase
  (:Pressed
    (Utilities|FlowControl|Gate true
      (:Exit
        (Utilities|ExecutionCheck) ; enters at B
      ))))

(fn ConstructionScript)
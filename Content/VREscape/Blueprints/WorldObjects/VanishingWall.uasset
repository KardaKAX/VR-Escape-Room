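; VanishingWall is a wall that can phase in and out, built on a parent property system.
; When IsVanishing is set, a timeline drives opacity on a dynamic material and enables collision only at full opacity.
; Tick watches for the suspended property to halt the timeline, using DoOnce gates to avoid repeated calls.
; Non-vanishing walls instead run parent setup, apply property material and effects, and record their initial scale.
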(event EventBeginPlay
  (bind _cube (Variables|Default|GetCube))
  ;[1 1 1] Check If Vanishing
  (if (Variables|Default|GetIsVanishing)
    ;[1 1 1] Timeline Affecting Material Opacity
    (bind _phasing (Timeline|Timeline_0 Play)
      (:Update
        (Rendering|Material|SetScalarParameterValue (Variables|Default|GetTranslucency) "Opacity" (Math|Float|Lerp 0.0 1.0 _phasing) :!class /Script/Engine.MaterialInstanceDynamic)
        (if (>= _phasing 1.0)
          (Collision|SetCollisionEnabled _cube "QueryAndPhysics")
          (else
            (Collision|SetCollisionEnabled _cube "NoCollision"))))
      (:Finished
        (Utilities|FlowControl|DoOnce false) ; enters at Reset
      ))
    (else
      (|CallParentFunction)
      (CallFunction|UpdatePropertyMaterial self (Variables|Default|GetCube) 0 false)
      (CallFunction|UpdatePropertyEffect)
      (CallFunction|PropertyEventScaleInit)
      (Variables|Default|SetinitialScaleEnum (Variables|Default|GetpropertyScale))
      (Variables|Default|SetinitialScale (Transformation|GetWorldScale (Variables|Default|GetCube))))))

(event EventTick
  (params (DeltaSeconds :type Float%20%28single-precision%29))
  (bind _cube (Variables|Default|GetCube))
  ;[1 1 1] Check If Suspended
  (if (Utilities|Enum|Equal(Enum) (Variables|Default|GetpropertyCurrent) "NewEnumerator8")
    ;[1 1 1] Timeline Affecting Material Opacity
    (Utilities|FlowControl|DoOnce false
      (:Completed
        (bind _phasing (Timeline|Timeline_0 Stop)
          (:Update
            (Rendering|Material|SetScalarParameterValue (Variables|Default|GetTranslucency) "Opacity" (Math|Float|Lerp 0.0 1.0 _phasing) :!class /Script/Engine.MaterialInstanceDynamic)
            (if (>= _phasing 1.0)
              (Collision|SetCollisionEnabled _cube "QueryAndPhysics")
              (else
                (Collision|SetCollisionEnabled _cube "NoCollision"))))
          (:Finished
            (goto _label Reset)))))
    (else
      (Utilities|FlowControl|DoOnce false :!label _label
        (:Completed
          (Timeline|Timeline_0 Play))))))

(fn ConstructionScript
  (|CallParentFunction)
  (if (Variables|Default|GetIsVanishing)
    (bind _returnvalue (Rendering|Material|CreateDynamicMaterialInstance (Variables|Default|GetCube) 0 (Rendering|Material|GetMaterial (Variables|Default|GetCube) 0) "Opacity" :!class /Script/Engine.PrimitiveComponent))
    (Variables|Default|SetTranslucency _returnvalue)))
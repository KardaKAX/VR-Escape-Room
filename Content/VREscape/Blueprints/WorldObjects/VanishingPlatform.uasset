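; VanishingPlatform is a VR escape world object: a platform that phases in opacity and is solid only when fully opaque.
; The construction script creates a dynamic material instance on the Cube and stores it as Translucency.
; On BeginPlay, a timeline's Phasing track drives that material's Opacity parameter each update, enabling query and physics collision at full value and disabling collision otherwise.
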(event EventBeginPlay
  (bind _cube (Variables|Default|GetCube))
  (bind _phasing (Timeline|Timeline_0 Play)
    (:Update
      (Rendering|Material|SetScalarParameterValue (Variables|Default|GetTranslucency) "Opacity" (Math|Float|Lerp 0.0 1.0 _phasing) :!class /Script/Engine.MaterialInstanceDynamic)
      (if (>= _phasing 1.0)
        (Collision|SetCollisionEnabled _cube "QueryAndPhysics")
        (else
          (Collision|SetCollisionEnabled _cube "NoCollision"))))))

(fn ConstructionScript
  (bind _returnvalue (Rendering|Material|CreateDynamicMaterialInstance (Variables|Default|GetCube) 0 (Rendering|Material|GetMaterial (Variables|Default|GetCube) 0) "Opacity" :!class /Script/Engine.PrimitiveComponent))
  (Variables|Default|SetTranslucency _returnvalue))
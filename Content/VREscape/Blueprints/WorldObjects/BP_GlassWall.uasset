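; BP_GlassWall is a breakable world object in VREscape that effect cubes can damage.
; When a BP_EffectCube overlaps the Box and a property check passes, accumulated damage rises and is applied as radius damage at the cube's location to an APEX destructible mesh.
; Each qualifying hit is stronger than the last, and once the mesh fractures the actor destroys itself after a short delay.
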(event OnComponentBeginOverlap(Box)
  (params (OverlappedComponent :type Primitive%20Component%20Object%20Reference) (OtherActor :type Actor%20Object%20Reference) (OtherComp :type Primitive%20Component%20Object%20Reference) (OtherBodyIndex :type Integer) (bFromSweep :type Boolean) (SweepResult :type Hit%20Result%20Structure%20%28by%20ref%29))
  (bind _asbp_effect_cube (Utilities|Casting|CastToBP_EffectCube OtherActor))
  (if (Utilities|Enum|Equal(Enum) (Variables|Default|GetpropertyCurrent) "NewEnumerator4")
    (bind _output_get (Variables|Default|SetDamage (+ (Variables|Default|GetDamage) 0.25)))
    (Class|DestructibleComponent|ApplyRadiusDamage (Variables|Default|Get1M_Cube_Apex_DM) _output_get (Transformation|GetActorLocation _asbp_effect_cube) 1e+02 1e+02 false)))

(event OnComponentFracture(1M_Cube_Apex_DM)
  (params (HitPoint :type Vector%20%28by%20ref%29 :default "0, 0, 0") (HitDirection :type Vector%20%28by%20ref%29 :default "0, 0, 0"))
  (Utilities|FlowControl|Delay 2.0)
  (Actor|DestroyActor))

(fn ConstructionScript
  (|CallParentFunction))
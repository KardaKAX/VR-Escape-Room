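; Sliding door actor for the VR escape game, opened and closed through its DoorOpen and DoorClose events.
; BeginPlay caches the start location and sets the timeline position to match the Open flag.
; The timeline lerps the actor between that location and an Offset from it without sweeping.
; Each event updates Open, plays its sound at the cached location, and runs the timeline forward or in reverse.
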(event Custom|DoorOpen
  (bind _location (Variables|Default|GetLocation))
  ;[1 1 1] Set door open
  (Variables|Default|SetOpen? true)
  ;[1 1 1] Sounds
  (Audio|PlaySoundatLocation "/Game/Audio/Door/DoorOpen.DoorOpen" (stale EventBeginPlay _output_get) "0, 0, 0" 1.0 1.0 0.0 "/Game/Audio/Door/DoorAttenuation.DoorAttenuation" 0 0)
  ;[1 1 1] Sets location
  (bind _newtrack_0 (Timeline|DoorTimeLine Play)
    (:Update
      (Transformation|SetActorLocation (Math|Vector|Lerp(Vector) _location (+ _location (Variables|Default|GetOffset)) _newtrack_0) false false))))

(event Custom|DoorClose
  (bind _location (Variables|Default|GetLocation))
  ;[1 1 1] Set door close
  (Variables|Default|SetOpen? false)
  ;[1 1 1] Sounds
  (Audio|PlaySoundatLocation "/Game/Audio/Door/DoorClose.DoorClose" (stale EventBeginPlay _output_get) "0, 0, 0" 1.0 1.0 0.0 "/Game/Audio/Door/DoorAttenuation.DoorAttenuation" 0 0)
  ;[1 1 1] Sets location
  (bind _newtrack_0 (Timeline|DoorTimeLine Reverse)
    (:Update
      (Transformation|SetActorLocation (Math|Vector|Lerp(Vector) _location (+ _location (Variables|Default|GetOffset)) _newtrack_0) false false))))

(event EventBeginPlay
  ;[1 1 1] Sets intial location
  (bind _output_get (Variables|Default|SetLocation (Transformation|GetActorLocation)))
  ;[1 1 1] Sets location
  (bind _newtrack_0 (Timeline|DoorTimeLine SetNewTime)
    (:Update
      (Transformation|SetActorLocation (Math|Vector|Lerp(Vector) (Variables|Default|GetLocation) (+ (Variables|Default|GetLocation) (Variables|Default|GetOffset)) _newtrack_0) false false))))

(fn ConstructionScript)
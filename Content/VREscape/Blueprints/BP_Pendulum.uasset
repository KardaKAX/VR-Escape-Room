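; Swinging pendulum puzzle prop with chains and a key card that the non-VR player can collect once the Suspend property is applied.
; The Suspend event toggles physics on chains and card, while Tick stops or loops their animation based on the current property.
; An overlap box enables input for PlayerNoVR, so pressing interact while suspended hides the card and grants the player the key.
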(event OnComponentBeginOverlap(Box1)
  (params (OverlappedComponent :type Primitive%20Component%20Object%20Reference) (OtherActor :type Actor%20Object%20Reference) (OtherComp :type Primitive%20Component%20Object%20Reference) (OtherBodyIndex :type Integer) (bFromSweep :type Boolean) (SweepResult :type Hit%20Result%20Structure%20%28by%20ref%29))
  ;[1 1 1] Enable/disable input
  (Utilities|Casting|CastToPlayerNoVR OtherActor)
  (Input|EnableInput (Game|GetPlayerController 0)))

(event OnComponentEndOverlap(Box1)
  (params (OverlappedComponent :type Primitive%20Component%20Object%20Reference) (OtherActor :type Actor%20Object%20Reference) (OtherComp :type Primitive%20Component%20Object%20Reference) (OtherBodyIndex :type Integer))
  ;[1 1 1] Enable/disable input
  (Utilities|Casting|CastToPlayerNoVR OtherActor)
  (Input|DisableInput (Game|GetPlayerController 0)))

(event Custom|propertyEvent_Suspend
  (params (isActive :type Boolean))
  ;[1 1 1] Suspend
  (Physics|SetSimulatePhysics (Variables|Default|GetChains) (not isActive))
  (Variables|Default|SetIsSuspended (Utilities|Enum|Equal(Enum) (Variables|Default|GetpropertyCurrent) "NewEnumerator8")))

(event EventTick
  (params (DeltaSeconds :type Float%20%28single-precision%29))
  (bind _chains (Variables|Default|GetChains))
  ;[1 1 1] Stop/Start Animation
  (if (Utilities|Enum|Equal(Enum) (Variables|Default|GetpropertyCurrent) "NewEnumerator8")
    (Audio|Components|Audio|Stop _chains)
    (else
      (Audio|Components|Audio|Play _chains true))))

(event Input|ActionEvents|InputActionFPSInteract
  (params (Key :type Key%20Structure))
  ;[1 1 1] PickUpCard
  (:Pressed
    (if (Utilities|Enum|Equal(Enum) (Variables|Default|GetpropertyCurrent) "NewEnumerator8")
      (Rendering|SetVisibility (Variables|Default|GetCard) false false)
      (bind _asplayer_no_vr (Utilities|Casting|CastToPlayerNoVR (Game|GetPlayerCharacter 0)))
      (Variables|/Game/VREscape/Characters/PlayerNoVR.PlayerNoVR_C|SetHasKey _asplayer_no_vr true))))

(fn ConstructionScript)
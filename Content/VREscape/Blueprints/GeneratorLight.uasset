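; GeneratorLight is a spotlight Blueprint in the VR escape game that lights up only while it is powered.
; BeginPlay hides the SpotLight, then Tick polls IsPowered after running the parent's logic.
; A DoOnce shows the light when power is present, and the unpowered branch hides it and resets the DoOnce each tick.
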(event EventBeginPlay
  ;[1 1 1] Set light visiblity false
  (|CallParentFunction)
  (Rendering|SetVisibility (Variables|Default|GetSpotLight) false false))

(event Collision|EventActorBeginOverlap
  (params (OtherActor :type Actor%20Object%20Reference))
  (|CallParentFunction OtherActor) ; This node is disabled and will not be called.\nDrag off pins to build functionality.
)

(event EventTick
  (params (DeltaSeconds :type Float%20%28single-precision%29))
  ;[1 1 1] Checks if have power and sets visibilty
  (|CallParentFunction DeltaSeconds)
  (if (Variables|Default|GetIsPowered?)
    (Utilities|FlowControl|DoOnce false :!label _label
      (:Completed
        (Rendering|SetVisibility (Variables|Default|GetSpotLight) true false)))
    (else
      (Utilities|FlowControl|Sequence
        (:then_0
          (Rendering|SetVisibility (Variables|Default|GetSpotLight) false false))
        (:then_1
          (goto _label Reset))))))

(fn ConstructionScript
  (|CallParentFunction))